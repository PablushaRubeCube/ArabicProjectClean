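; BP_TradeHouses is an environment actor that fills a square grid with trade houses.
; Its construction script runs nested loops, adding a child actor component at each cell, spaced by a size value, and setting its class to BP_TradeHouse.
; Each house gets a random yaw in multiples of a rotator value, using an unseeded roll, so orientations can change whenever construction reruns.
; The event graph holds no active logic.
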(event EventBeginPlay)

(event Collision|EventActorBeginOverlap
  (params (OtherActor :type Actor%20Object%20Reference)))

(event EventTick
  (params (DeltaSeconds :type Float%20%28single-precision%29)))

(fn ConstructionScript
  (bind _index (Variables|Default|GetIndex))
  (for _index_2 (range 0 _index)
    (for _index_3 (range 0 _index)
      (bind _returnvalue (AddComponent|AddChildActorComponent false (Math|Transform|MakeTransform (Math|Vector|MakeVector (* _index_3 (Variables|Default|GetSize)) (* (Math|Conversions|ToFloat(Integer) _index_2) (Variables|Default|GetSize)) 0.0) (Math|Rotator|MakeRotator 0.0 0.0 (* (Variables|Default|GetRotator) (Math|Random|RandomIntegerinRange 0 4))) "1.000000,1.000000,1.000000")))
      (Utilities|IsValid _returnvalue
        (:Is%20Valid
          (ChildActorComponent|SetChildActorClass _returnvalue "/Game/_ChibaChaba/Enviroment/BP_TradeHouse.BP_TradeHouse_C"))))))