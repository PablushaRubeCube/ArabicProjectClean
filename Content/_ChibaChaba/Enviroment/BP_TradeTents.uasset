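; BP_TradeTents lays out a row of randomly chosen actors, apparently trade tents, along its forward vector.
; The construction script adds child actor components at 1000-unit steps up to LastIndex, each taking a random entry from the Class array.
; Absolute location and rotation place them in world space, independent of the parent's rotation.
; BeginPlay is empty, and an older runtime SpawnActor loop is left disconnected.
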(event EventBeginPlay)

(fn ConstructionScript
  (for _index (range 0 (Variables|Default|GetLast%20Index))
    (bind _returnvalue (AddComponent|AddChildActorComponent false (Math|Transform|MakeTransform (+ (* (* _index 1000) (Math|Vector|Normalize (Transformation|GetActorForwardVector))) (Transformation|GetActorLocation)) "0, 0, 0" "1.000000,1.000000,1.000000")))
    (Utilities|IsValid _returnvalue
      (:Is%20Valid
        (ChildActorComponent|SetChildActorClass _returnvalue (.OutItem (Utilities|Array|Random (Variables|Default|GetClass))))
        (Transformation|SetAbsolute _returnvalue true true false)))))