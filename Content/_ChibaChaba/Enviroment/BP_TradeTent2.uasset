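; BP_TradeTent2 is an environment Blueprint that builds a square floor grid of static mesh tiles in its construction script, with no active event logic.
; Nested loops share one upper bound and add a component per cell, spaced along X and Y by Size.
; Each tile gets a random Floor array mesh; the random pick is pure, so the validity check and the assignment can select different entries.
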(event EventBeginPlay)

(event Collision|EventActorBeginOverlap
  (params (OtherActor :type Actor%20Object%20Reference)))

(event EventTick
  (params (DeltaSeconds :type Float%20%28single-precision%29)))

(fn ConstructionScript
  (bind _floor (Variables|Default|GetFloor))
  (bind _index (Variables|Default|GetIndex))
  (bind _floor_2 (Variables|Default|GetFloor))
  (bind _returnvalue (Utilities|Array|Length _floor_2))
  (bind _returnvalue_2 (- _returnvalue 1))
  (bind _returnvalue_3 (Math|Random|RandomIntegerinRange 0 _returnvalue_2))
  (bind _output (Utilities|Array|Get(acopy) _floor _returnvalue_3))
  (for _index_2 (range 0 _index)
    (for _index_3 (range 0 _index)
      (bind _returnvalue_4 (AddComponent|AddStaticMeshComponent false (Math|Transform|MakeTransform (Math|Vector|MakeVector (Math|Conversions|ToFloat(Integer) (* _index_2 (Variables|Default|GetSize))) (Math|Conversions|ToFloat(Integer) (* _index_3 (Variables|Default|GetSize))) 0.0) "0, 0, 0" "1.000000,1.000000,1.000000")))
      (Utilities|IsValid _returnvalue_4
        (:Is%20Valid
          (Utilities|IsValid _output
            (:Is%20Valid
              (Components|StaticMesh|SetStaticMesh _returnvalue_4 _output))))))))