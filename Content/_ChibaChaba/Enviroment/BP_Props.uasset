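; Environment prop actor that builds static mesh floor pieces in its construction script, drawing meshes at random from the Floor array.
; Nested loops place rotated mesh components on a grid spaced by SizeProps, though the current bounds yield only one piece at the origin.
; The random pick is made separately for the validity check and the mesh assignment, and the event graph has no active logic.
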(event EventBeginPlay)

(event Collision|EventActorBeginOverlap
  (params (OtherActor :type Actor%20Object%20Reference)))

(event EventTick
  (params (DeltaSeconds :type Float%20%28single-precision%29)))

(fn ConstructionScript
  (bind _floor (Variables|Default|GetFloor))
  (bind _floor_2 (Variables|Default|GetFloor))
  (bind _returnvalue (Utilities|Array|Length _floor_2))
  (bind _returnvalue_2 (- _returnvalue 1))
  (bind _returnvalue_3 (Math|Random|RandomIntegerinRange 0 _returnvalue_2))
  (bind _output (Utilities|Array|Get(acopy) _floor _returnvalue_3))
  (for _index (range 0 0)
    (for _index_2 (range 0 (Variables|Default|GetIndex))
      (bind _returnvalue_4 (AddComponent|AddStaticMeshComponent false (Math|Transform|MakeTransform (Math|Vector|MakeVector (Math|Conversions|ToFloat(Integer) (* _index (Variables|Default|GetSizeProps))) (Math|Conversions|ToFloat(Integer) (* _index_2 (Variables|Default|GetSizeProps))) 0.0) "0.000000,90.000000,0.000000" "1.000000,1.000000,1.000000")))
      (Utilities|IsValid _returnvalue_4
        (:Is%20Valid
          (Utilities|IsValid _output
            (:Is%20Valid
              (Components|StaticMesh|SetStaticMesh _returnvalue_4 _output))))))))