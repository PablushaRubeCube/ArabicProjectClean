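; Magic bolt spell projectile that flies along its local axes and damages the first enemy it overlaps.
; MakeShoot takes the shot characteristics, matches the Niagara effect and Shoot timeline to the lifetime, and moves the actor each update by a speed-scaled offset without sweep.
; Enemy overlaps are forwarded to the owning BP_BaseWeapon, then the bolt destroys itself; it also destroys itself when the timeline finishes.
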(event Custom|MakeShoot
  (params (Characteristics :type Weapon%20Characteristics%20Structure))
  (bind _niagara (Variables|Default|GetNiagara))
  (bind _shoot (Variables|Default|GetShoot))
  (Utilities|IsValid _niagara
    (:Is%20Valid
      ;[1 1 1] Setup param. Play shoot
      (Effects|Components|ParticleSystem|SetFloatParameter _niagara "LifeTime" (.lifetime Characteristics))
      (Utilities|IsValid _shoot
        (:Is%20Valid
          (Components|Timeline|SetTimelineLength _shoot (.lifetime Characteristics))
          (Timeline|Shoot Play
            (:Update
              (Transformation|AddActorLocalOffset self (* (.speed Characteristics) (Variables|Default|GetDelta%20Location)) false false))
            (:Finished
              (Actor|DestroyActor))))))))

(event Collision|EventActorBeginOverlap
  (params (OtherActor :type Actor%20Object%20Reference))
  (bind _returnvalue (Components|GetOwner))
  ;[1 1 1] Damage char
  (Utilities|Casting|CastToEnemyCharacter OtherActor)
  (Utilities|IsValid _returnvalue
    (:Is%20Valid
      (bind _asbp_base_weapon (Utilities|Casting|CastToBP_BaseWeapon _returnvalue))
      (Utilities|IsValid _asbp_base_weapon
        (:Is%20Valid
          (Class|BaseWeapon|OnActorWeaponOverlap _asbp_base_weapon 0 OtherActor)
          (Actor|DestroyActor))))))

(fn ConstructionScript)