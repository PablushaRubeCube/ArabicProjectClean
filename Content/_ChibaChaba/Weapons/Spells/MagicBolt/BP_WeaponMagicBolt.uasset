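; BP_WeaponMagicBolt is the Magic Bolt spell weapon, which fires repeating volleys of projectiles.
; SetupEffects sets the StartShoot timeline's length to the reload rate, using it as the cooldown before a looping timer starts.
; Each timer tick plays a sound and spawns an unpooled BP_WeaponProjectileMagicBolt at fixed height, passing it the weapon's characteristics.
; Once Quantity bolts have spawned, it clears the timer and restarts the timeline.
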(event Custom|CustomEvent
  (bind _returnvalue (Transformation|GetActorTransform))
  ;[1 1 1] setup and start weapon logic
  (Audio|PlaySound2D (Variables|Default|GetInitSound) 1.0 1.0 0.0 0 0)
  ;;[1 1 1] TODO pool magic bolt
  (bind _returnvalue_2 (Game|SpawnActorfromClass "/Game/_ChibaChaba/Weapons/Spells/MagicBolt/BP_WeaponProjectileMagicBolt.BP_WeaponProjectileMagicBolt_C" (Math|Transform|MakeTransform (Math|Vector|MakeVector (.x (.location _returnvalue)) (.y (.location _returnvalue)) 9e+01) (.rotation _returnvalue) (.scale _returnvalue)) "AlwaysSpawn" "MultiplyWithRoot" self 0))
  (Utilities|IsValid _returnvalue_2
    (:Is%20Valid
      (Default|MakeShoot _returnvalue_2 (Variables|Default|GetWeaponCurrentCharacteristics))
      (bind _result (Math|Integer|IncrementInt (Variables|Default|GetCount))
        (:%20%20
          (if (>= _result (.quantity (Variables|Default|GetWeaponCurrentCharacteristics)))
            (Variables|Default|SetCount 0)
            (Utilities|Time|ClearandInvalidateTimerbyHandle (stale _returnvalue_3))
            (Timeline|StartShoot PlayFromStart
              (:Finished
                (bind _returnvalue_3 (Utilities|Time|SetTimerbyEvent (delegate Custom|CustomEvent) 0.2 true))))))))))

(event EventBeginPlay
  (|CallParentFunction))

(event EventSetupEffects
  (bind _startshoot (Variables|Default|GetStartShoot))
  ;[1 1 1] setup and start weapon logic
  (Utilities|IsValid _startshoot
    (:Is%20Valid
      (Components|Timeline|SetTimelineLength _startshoot (.reloadrate (Variables|Default|GetWeaponCurrentCharacteristics)))
      (Timeline|StartShoot Play
        (:Finished
          (bind _returnvalue (Utilities|Time|SetTimerbyEvent (delegate Custom|CustomEvent) 0.2 true)))))))

(event EventTick
  (params (DeltaSeconds :type Float%20%28single-precision%29))
  (|CallParentFunction DeltaSeconds))

(event Collision|EventActorBeginOverlap
  (params (OtherActor :type Actor%20Object%20Reference))
  (|CallParentFunction OtherActor) ; This node is disabled and will not be called.\nDrag off pins to build functionality.
)

(fn ConstructionScript
  (|CallParentFunction))