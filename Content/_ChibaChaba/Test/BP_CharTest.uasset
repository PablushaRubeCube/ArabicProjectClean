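; Test character Blueprint that handles enemy attack range and camera transitions tied to the game state.
; Its AttackSphere overlaps set a can-attack Blackboard flag on EnemyCharacters as they enter and leave.
; It binds to the ChibaChaba game mode's state change, showing the health widget only while in progress.
; Timelines ease GameCamera toward the inactive ToggleCamera's transform on start and back to its saved transform on game over.
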(event OnComponentBeginOverlap(AttackSphere)
  (params (OverlappedComponent :type Primitive%20Component%20Object%20Reference) (OtherActor :type Actor%20Object%20Reference) (OtherComp :type Primitive%20Component%20Object%20Reference) (OtherBodyIndex :type Integer) (bFromSweep :type Boolean) (SweepResult :type Hit%20Result%20Structure%20%28by%20ref%29))
  ;[1 1 1] TODO migrate to c++?
  ;;[1 1 1] AI Attack logic
  (bind _asenemy_character (Utilities|Casting|CastToEnemyCharacter OtherActor))
  (Utilities|IsValid (AI|GetBlackboard _asenemy_character)
    (:Is%20Valid
      (AI|Components|Blackboard|SetValueasBool (AI|GetBlackboard _asenemy_character) (Variables|Default|GetNameCanAttack?) true))))

(event OnComponentEndOverlap(AttackSphere)
  (params (OverlappedComponent :type Primitive%20Component%20Object%20Reference) (OtherActor :type Actor%20Object%20Reference) (OtherComp :type Primitive%20Component%20Object%20Reference) (OtherBodyIndex :type Integer))
  ;[1 1 1] TODO migrate to c++?
  ;;[1 1 1] AI Attack logic
  (bind _asenemy_character (Utilities|Casting|CastToEnemyCharacter OtherActor))
  (Utilities|IsValid (AI|GetBlackboard _asenemy_character)
    (:Is%20Valid
      (AI|Components|Blackboard|SetValueasBool (AI|GetBlackboard _asenemy_character) (Variables|Default|GetNameCanAttack?) false))))

(event Custom|OnChangeGameState_Event
  (params (State :type EGameStates%20Enum :default "EGS_WaitToStart"))
  ;[1 1 1] Trasform cameras when game start and end
  (switch Utilities|FlowControl|Switch|SwitchonEGameStates State
    (:EGS_InProgress
      ;;[1 1 1] toggle health widget
      (Rendering|SetVisibility (Variables|Default|GetHealthWidgetComponent) true false)
      (bind _newtrack_0 (Timeline|Timeline PlayFromStart)
        (:Update
          (Transformation|SetRelativeTransform (Variables|Default|GetGameCamera) (Class|KismetMathLibrary|TInterpto (Transformation|GetRelativeTransform (Variables|Default|GetGameCamera)) (Transformation|GetRelativeTransform (Variables|Default|GetToggleCamera)) _newtrack_0 1.0) false false))))
    (:EGS_GameOver
      (Rendering|SetVisibility (Variables|Default|GetHealthWidgetComponent) false false)
      (bind _newtrack_0_2 (Timeline|Timeline_0 PlayFromStart)
        (:Update
          (Transformation|SetRelativeTransform (Variables|Default|GetGameCamera) (Class|KismetMathLibrary|TInterpto (Transformation|GetRelativeTransform (Variables|Default|GetGameCamera)) (Variables|Default|GetRestartCameraTransform) _newtrack_0_2 1.0) false true))))))

(event EventBeginPlay
  (bind _returnvalue (Game|GetGameMode))
  ;[1 1 1] Trasform cameras when game start and end
  (Variables|Default|SetRestartCameraTransform (Transformation|GetRelativeTransform (Variables|Default|GetGameCamera)))
  ;;[1 1 1] toggle health widget
  (Rendering|SetVisibility (Variables|Default|GetHealthWidgetComponent) false false)
  (Components|Activation|SetActive (Variables|Default|GetToggleCamera) false false)
  (Components|Activation|SetActive (Variables|Default|GetGameCamera) true false)
  (Utilities|IsValid _returnvalue
    (:Is%20Valid
      (bind _aschiba_chaba_game_mode_base (Utilities|Casting|CastToChibaChabaGameModeBase _returnvalue))
      (EventDispatchers|AssignOnChangeGameState _aschiba_chaba_game_mode_base (delegate Custom|OnChangeGameState_Event)))))

(fn ConstructionScript)